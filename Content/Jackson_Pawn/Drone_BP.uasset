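; Player-controlled drone pawn that flies with WASD, Space and Left Ctrl and looks around with the mouse.
; Each held key runs a looping frame-delta timer that feeds directional input into FloatingPawnMovement, with forward and backward flattened to horizontal.
; Mouse input yaws the Cube component and sets its clamped pitch.
; Tick restarts a camera shake every frame; the custom shake functions are uncalled, and ApplyShake is empty.
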(event `Key|W`
  (params (Key :type "Key Structure"))
  (:`Pressed`
    (bind _returnvalue (`KismetSystemLibrary.K2_SetTimerDelegate` (delegate `Forward`) (`GameplayStatics.GetWorldDeltaSeconds`) true)))
  (:`Released`
    (`KismetSystemLibrary.K2_ClearAndInvalidateTimerHandle` _returnvalue)))

(event `Forward`
  (`PawnMovementComponent.AddInputVector` (`self.FloatingPawnMovement`) (`KismetMathLibrary.Vector_Normal2D` (`self.GetActorForwardVector`)) false))

(event `Key|S`
  (params (Key :type "Key Structure"))
  (:`Pressed`
    (bind _returnvalue (`KismetSystemLibrary.K2_SetTimerDelegate` (delegate `Backward`) (`GameplayStatics.GetWorldDeltaSeconds`) true)))
  (:`Released`
    (`KismetSystemLibrary.K2_ClearAndInvalidateTimerHandle` _returnvalue)))

(event `Backward`
  (`PawnMovementComponent.AddInputVector` (`self.FloatingPawnMovement`) (`KismetMathLibrary.Vector_Normal2D` (* (`self.GetActorForwardVector`) -1.0)) false))

(event `Key|D`
  (params (Key :type "Key Structure"))
  (:`Pressed`
    (bind _returnvalue (`KismetSystemLibrary.K2_SetTimerDelegate` (delegate `Right`) (`GameplayStatics.GetWorldDeltaSeconds`) true)))
  (:`Released`
    (`KismetSystemLibrary.K2_ClearAndInvalidateTimerHandle` _returnvalue)))

(event `Right`
  (`PawnMovementComponent.AddInputVector` (`self.FloatingPawnMovement`) (`self.GetActorRightVector`) false))

(event `Key|A`
  (params (Key :type "Key Structure"))
  (:`Pressed`
    (bind _returnvalue (`KismetSystemLibrary.K2_SetTimerDelegate` (delegate `Left`) (`GameplayStatics.GetWorldDeltaSeconds`) true)))
  (:`Released`
    (`KismetSystemLibrary.K2_ClearAndInvalidateTimerHandle` _returnvalue)))

(event `Left`
  (`PawnMovementComponent.AddInputVector` (`self.FloatingPawnMovement`) (* (`self.GetActorRightVector`) -1.0) false))

(event `Key|SpaceBar`
  (params (Key :type "Key Structure"))
  (:`Pressed`
    (bind _returnvalue (`KismetSystemLibrary.K2_SetTimerDelegate` (delegate `Ascend`) (`GameplayStatics.GetWorldDeltaSeconds`) true)))
  (:`Released`
    (`KismetSystemLibrary.K2_ClearAndInvalidateTimerHandle` _returnvalue)))

(event `Ascend`
  (`PawnMovementComponent.AddInputVector` (`self.FloatingPawnMovement`) (0.0 0.0 1.0) false))

(event `Key|LeftControl`
  (params (Key :type "Key Structure"))
  (:`Pressed`
    (bind _returnvalue (`KismetSystemLibrary.K2_SetTimerDelegate` (delegate `Descend`) (`GameplayStatics.GetWorldDeltaSeconds`) true)))
  (:`Released`
    (`KismetSystemLibrary.K2_ClearAndInvalidateTimerHandle` _returnvalue)))

(event `self.ReceiveTick`
  (params (DeltaSeconds :type "Float (single-precision)"))
  (`CameraShakeSourceComponent.StartCameraShake` :`self` (`self.CameraShakeSource`) :`InCameraShake` "/Game/NewBlueprint.NewBlueprint_C" :`Scale` 5.0))

(event `Descend`
  (`PawnMovementComponent.AddInputVector` (`self.FloatingPawnMovement`) (0.0 0.0 -1.0) false))

(event `InputAxisKey|MouseX`
  (params (AxisValue :type "Float (single-precision)"))
  (`SceneComponent.K2_AddWorldRotation` (`self.Cube`) (`KismetMathLibrary.MakeRotator` 0.0 0.0 AxisValue) false false))

(event `InputAxisKey|MouseY`
  (params (AxisValue :type "Float (single-precision)"))
  (bind (_relativerotation_roll _relativerotation_pitch _relativerotation_yaw) (`KismetMathLibrary.BreakRotator` (`SceneComponent.RelativeRotation` (`self.Cube`))))
  (`SceneComponent.K2_SetRelativeRotation` (`self.Cube`) (`KismetMathLibrary.MakeRotator` _relativerotation_roll (`KismetMathLibrary.FClamp` (+ AxisValue _relativerotation_pitch) -88.0 88.0) _relativerotation_yaw) false false))

(fn `Apply Shake`)

(fn `Set new random vector`
  (returns (`New float` :type "Vector Structure"))
  (bind _returnvalue (`KismetMathLibrary.RandomUnitVector`))
  (set `self.Drone Shake` _returnvalue)
  (set `self.Start Shake` (0.0 0.0 0.0))
  (return _returnvalue))

(fn `UserConstructionScript`)